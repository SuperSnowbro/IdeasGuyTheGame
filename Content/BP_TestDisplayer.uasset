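; Text display actor that reveals its DisplayText in a TextRender component one character at a time, typewriter style.
; The construction script scales the Pivot from TextBoxScale with remapped axes, then inserts <br> breaks using a line limit derived from box width and font scale.
; Tick uses a Delay to advance the visible substring roughly every tenth of a second, skipping over each <br> tag as a whole.
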(event `self.ReceiveTick`
  (params (DeltaSeconds :type "Float (single-precision)"))
  (`KismetSystemLibrary.Delay` 0.1)
  (`/Engine/EditorBlueprintResources/StandardMacros.IncrementInt` (`self.DisplayNumberOfChars`)
    (:`  `
      (`self.UpdateDisplayText`))))

(fn `BreakStringIntoLines`
  (params (String :type String) (MaxCharacters :type Integer))
  (returns (BrokenString :type String))
  (locals (CharactersPerLine :type Integer) (Result :type String) (Counter :type Integer) (CurrentArrayWord :type String))
  (bind _result (`local.Result`))
  (set `local.CharactersPerLine` MaxCharacters)
  (for _array_element (`KismetStringLibrary.ParseIntoArray` String)
    (set `local.CurrentArrayWord` _array_element)
    (bind _output_get (set `local.Counter` (+ (`local.Counter`) (`KismetStringLibrary.Len` _array_element))))
    (if (>= _output_get (`local.CharactersPerLine`))
      (set `local.Result` (`KismetStringLibrary.Concat_StrStr` (`local.Result`) "<br>"))
      (set `local.Counter` (`KismetStringLibrary.Len` (`local.CurrentArrayWord`)))
      (set `local.Result` (`KismetStringLibrary.Concat_StrStr` (`local.Result`) (`local.CurrentArrayWord`)))
      (else
        (set `local.Result` (`KismetStringLibrary.Concat_StrStr` (`local.Result`) " " (`local.CurrentArrayWord`))))))
  (return (`KismetStringLibrary.GetSubstring` _result 1 (`KismetStringLibrary.Len` _result))))

(fn `ScaleAdjustment`
  (params (NormalScale :type "Vector Structure"))
  (returns (CorrectedFuckedUpScale :type "Vector Structure"))
  (return (`KismetMathLibrary.MakeVector` NormalScale_Z NormalScale_X 1.0)))

(fn `UpdateDisplayText`
  (if (== (`KismetStringLibrary.FindSubstring` (`self.ElaboratedText`) "<br>" false false (`self.DisplayNumberOfChars`)) (`self.DisplayNumberOfChars`))
    (set `self.DisplayNumberOfChars` (+ (`self.DisplayNumberOfChars`) (`KismetStringLibrary.Len` "<br>"))))
  (`TextRenderComponent.K2_SetText` (`self.TextRender`) (`KismetTextLibrary.Conv_StringToText` (`KismetStringLibrary.GetSubstring` (`self.ElaboratedText`) 0 (`self.DisplayNumberOfChars`)))))

(fn `UserConstructionScript`
  (bind (_textboxscale_x _textboxscale_y) (`KismetMathLibrary.BreakVector2D` (`self.TextBoxScale`)))
  (bind _textboxscale_x_2 (`KismetMathLibrary.BreakVector2D` (`self.TextBoxScale`)))
  (`SceneComponent.SetRelativeScale3D` (`self.Pivot`) (`self.ScaleAdjustment` (`KismetMathLibrary.MakeVector` _textboxscale_x 1.0 _textboxscale_y)))
  (bind _brokenstring (`self.BreakStringIntoLines` (`self.DisplayText`) (`KismetMathLibrary.FTrunc` (* _textboxscale_x_2 21.0 (/ 1.0 (`TextRenderComponent.XScale` (`self.TextRender`))) (/ 10.0 (`TextRenderComponent.WorldSize` (`self.TextRender`)))))))
  (bind _output_get (set `self.ElaboratedText` _brokenstring))
  (`TextRenderComponent.K2_SetText` (`self.TextRender`) (`KismetTextLibrary.Conv_StringToText` _output_get)))